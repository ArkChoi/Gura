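; Arcade room player controller that manages three on-screen widgets: punch, item obtain and light.
; Events add and remove the widgets, creating them on the authority side only for controller ID 0, or directly on remote controllers.
; The IA_Optain input swaps an active obtain widget for the light widget with cursor and Game-and-UI input, or closes an open light widget and restores game-only input.
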(event Custom|AddOptainItemWidget
  ;[0.15 0.15 0.15 0.5] Comment
  (Networking|SwitchHasAuthority
    (:Authority
      (if (== (Class|GameplayStatics|GetPlayerControllerID self) 0)
        (bind _returnvalue (UserInterface|CreateWidget "/Game/BluePrint/BPHUD/WBP_OptainItem.WBP_OptainItem_C"))
        (bind _output_get (Variables|Default|SetOptainWidget _returnvalue))
        (UserInterface|Viewport|AddtoViewport _output_get 0)))
    (:Remote
      (bind _returnvalue_2 (UserInterface|CreateWidget "/Game/BluePrint/BPHUD/WBP_OptainItem.WBP_OptainItem_C"))
      (bind _output_get_2 (Variables|Default|SetOptainWidget _returnvalue_2))
      (UserInterface|Viewport|AddtoViewport _output_get_2 0))))

(event Custom|AddPunchWidget
  ;[0.15 0.15 0.15 0.5] Comment
  (Utilities|IsValid (Variables|Default|GetPunchWidget)
    (:Is%20Not%20Valid
      (Networking|SwitchHasAuthority
        (:Authority
          (if (== (Class|GameplayStatics|GetPlayerControllerID self) 0)
            (bind _returnvalue (UserInterface|CreateWidget "/Game/BluePrint/BPHUD/ArcadeRoom/WBP_PunchWidget.WBP_PunchWidget_C"))
            (bind _output_get (Variables|Default|SetPunchWidget _returnvalue))
            (UserInterface|Viewport|AddtoViewport _output_get 0)))
        (:Remote
          (bind _returnvalue_2 (UserInterface|CreateWidget "/Game/BluePrint/BPHUD/ArcadeRoom/WBP_PunchWidget.WBP_PunchWidget_C"))
          (bind _output_get_2 (Variables|Default|SetPunchWidget _returnvalue_2))
          (UserInterface|Viewport|AddtoViewport _output_get_2 0))))))

(event Custom|AddLightWidget
  ;[0.15 0.15 0.15 0.5] Comment
  (Networking|SwitchHasAuthority
    (:Authority
      (if (== (Class|GameplayStatics|GetPlayerControllerID self) 0)
        (bind _returnvalue (UserInterface|CreateWidget "/Game/BluePrint/BPHUD/ArcadeRoom/WBP_Light.WBP_Light_C"))
        (bind _output_get (Variables|Default|SetLightWidget _returnvalue))
        (UserInterface|Viewport|AddtoViewport _output_get 0)))
    (:Remote
      (bind _returnvalue_2 (UserInterface|CreateWidget "/Game/BluePrint/BPHUD/ArcadeRoom/WBP_Light.WBP_Light_C"))
      (bind _output_get_2 (Variables|Default|SetLightWidget _returnvalue_2))
      (UserInterface|Viewport|AddtoViewport _output_get_2 0))))

(event Custom|RemovePunchWidget
  ;[0.15 0.15 0.15 0.5] Comment
  (Networking|SwitchHasAuthority
    (:Authority
      (if (== (Class|GameplayStatics|GetPlayerControllerID self) 0)
        (Widget|RemovefromParent (Variables|Default|GetPunchWidget))
        (Variables|Default|SetPunchWidget 0)))
    (:Remote
      (Widget|RemovefromParent (Variables|Default|GetPunchWidget))
      (Variables|Default|SetPunchWidget 0))))

(event Custom|RemoveOptainItemWidget
  ;[0.15 0.15 0.15 0.5] Comment
  (Utilities|IsValid (Variables|Default|GetOptainWidget)
    (:Is%20Valid
      (Networking|SwitchHasAuthority
        (:Authority
          (if (== (Class|GameplayStatics|GetPlayerControllerID self) 0)
            (Widget|RemovefromParent (Variables|Default|GetOptainWidget))
            (Variables|Default|SetOptainWidget 0)))
        (:Remote
          (Widget|RemovefromParent (Variables|Default|GetOptainWidget))
          (Variables|Default|SetOptainWidget 0))))))

(event Input|EnhancedActionEvents|EnhancedInputActionIA_Optain
  (params (ActionValue :type Boolean) (ElapsedSeconds :type Float%20%28double-precision%29) (TriggeredSeconds :type Float%20%28double-precision%29) (InputAction :type Input%20Action%20Object%20Reference :default "/Game/Input/Actions/IA_Optain.IA_Optain"))
  ;[0.15 0.15 0.15 0.5] Comment
  (Utilities|IsValid (Variables|Default|GetLightWidget)
    (:Is%20Valid
      ;;[0.15 0.15 0.15 0.5] Comment
      (Networking|SwitchHasAuthority
        (:Authority
          (if (== (Class|GameplayStatics|GetPlayerControllerID self) 0)
            (Widget|RemovefromParent (Variables|Default|GetLightWidget))
            (Variables|Default|SetbShowMouseCursor false)
            (Input|SetInputModeGameOnly self false)
            (Variables|Default|SetLightWidget 0)))
        (:Remote
          (Widget|RemovefromParent (Variables|Default|GetLightWidget))
          (Variables|Default|SetbShowMouseCursor false)
          (Input|SetInputModeGameOnly self false)
          (Variables|Default|SetLightWidget 0))))
    (:Is%20Not%20Valid
      (Utilities|IsValid (Variables|Default|GetOptainWidget)
        (:Is%20Valid
          (CallFunction|RemoveOptainItemWidget)
          (CallFunction|AddLightWidget)
          (Variables|Default|SetbShowMouseCursor true)
          (Input|SetInputModeGameandUI self 0 "DoNotLock" true false))))))

(fn ConstructionScript)