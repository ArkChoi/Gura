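; Player controller in the Gura folder that shows and hides the punch and item-obtain ("Optain") UI widgets.
; Paired add and remove events store each widget and toggle it on the viewport.
; Each splits on authority: remote instances act directly, while authority instances act only for controller ID 0, apparently targeting the host's local player.
; The IA_Optain input only prints a placeholder debug string while the obtain widget reference is valid.
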(event Custom|AddPunchWidget
  ;[0.15 0.15 0.15 0.5] Comment
  (Networking|SwitchHasAuthority
    (:Authority
      (if (== (Class|GameplayStatics|GetPlayerControllerID self) 0)
        (bind _returnvalue (UserInterface|CreateWidget "/Game/BluePrint/BPHUD/ArcadeRoom/WBP_PunchWidget.WBP_PunchWidget_C"))
        (bind _output_get (Variables|Default|SetPunchWidget _returnvalue))
        (UserInterface|Viewport|AddtoViewport _output_get 0)))
    (:Remote
      (bind _returnvalue_2 (UserInterface|CreateWidget "/Game/BluePrint/BPHUD/ArcadeRoom/WBP_PunchWidget.WBP_PunchWidget_C"))
      (bind _output_get_2 (Variables|Default|SetPunchWidget _returnvalue_2))
      (UserInterface|Viewport|AddtoViewport _output_get_2 0))))

(event Custom|AddOptainItemWidget
  ;[0.15 0.15 0.15 0.5] Comment
  (Networking|SwitchHasAuthority
    (:Authority
      (if (== (Class|GameplayStatics|GetPlayerControllerID self) 0)
        (bind _returnvalue (UserInterface|CreateWidget "/Game/BluePrint/BPHUD/WBP_OptainItem.WBP_OptainItem_C"))
        (bind _output_get (Variables|Default|SetOptainWidget _returnvalue))
        (UserInterface|Viewport|AddtoViewport _output_get 0)))
    (:Remote
      (bind _returnvalue_2 (UserInterface|CreateWidget "/Game/BluePrint/BPHUD/WBP_OptainItem.WBP_OptainItem_C"))
      (bind _output_get_2 (Variables|Default|SetOptainWidget _returnvalue_2))
      (UserInterface|Viewport|AddtoViewport _output_get_2 0))))

(event Custom|RemovePunchWidget
  ;[0.15 0.15 0.15 0.5] Comment
  (Networking|SwitchHasAuthority
    (:Authority
      (if (== (Class|GameplayStatics|GetPlayerControllerID self) 0)
        (Widget|RemovefromParent (Variables|Default|GetPunchWidget))))
    (:Remote
      (Widget|RemovefromParent (Variables|Default|GetPunchWidget)))))

(event Custom|RemoveOptainItemWidget
  ;[0.15 0.15 0.15 0.5] Comment
  (Networking|SwitchHasAuthority
    (:Authority
      (if (== (Class|GameplayStatics|GetPlayerControllerID self) 0)
        (Widget|RemovefromParent (Variables|Default|GetOptainWidget))))
    (:Remote
      (Widget|RemovefromParent (Variables|Default|GetOptainWidget)))))

(event Input|EnhancedActionEvents|EnhancedInputActionIA_Optain
  (params (ActionValue :type Boolean) (ElapsedSeconds :type Float%20%28double-precision%29) (TriggeredSeconds :type Float%20%28double-precision%29) (InputAction :type Input%20Action%20Object%20Reference :default "/Game/Input/Actions/IA_Optain.IA_Optain"))
  (:Triggered
    (Utilities|IsValid (Variables|Default|GetOptainWidget)
      (:Is%20Valid
        (Development|PrintString "Hello")))))

(fn ConstructionScript)