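; BP_SafeChangeActor is an overlap-triggered room actor that clears the "Punch" lighting and UI.
; When any actor begins overlapping it, it searches all SpotLights and hides the light component of those whose display name contains "Punch".
; If the overlapping actor is a BP_PCPuppet controlled by BP_ArcadeRoomPlayerController, it then calls RemovePunchWidget on that controller.
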(event Collision|EventActorBeginOverlap
  (params (OtherActor :type Actor%20Object%20Reference))
  (Utilities|FlowControl|Sequence
    (:then_0
      (bind _outactors (Actor|GetAllActorsOfClass "/Script/Engine.SpotLight"))
      (for _array_element _outactors
        (if (Utilities|String|Contains (Utilities|GetDisplayName _array_element) "Punch")
          (Rendering|SetVisibility (Variables|/Script/Engine.Light|GetLightComponent _array_element) false false))))
    (:then_1
      (bind _asbp_pcpuppet (Utilities|Casting|CastToBP_PCPuppet OtherActor))
      (bind _asbp_arcade_room_player_controller (Utilities|Casting|CastToBP_ArcadeRoomPlayerController (Pawn|GetController _asbp_pcpuppet)))
      (Default|RemovePunchWidget _asbp_arcade_room_player_controller))))

(fn ConstructionScript)