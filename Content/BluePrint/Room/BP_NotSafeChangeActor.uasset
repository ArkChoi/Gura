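; BP_NotSafeChangeActor is an overlap-triggered actor that activates the punch widget and punch lighting in the arcade room.
; On overlap, it adds the punch widget through the arcade room player controller of an overlapping BP_PCPuppet.
; It then searches all SpotLights and shows those whose display name contains "Punch".
; The lighting step runs for any overlapping actor, independent of the pawn and controller casts.
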(event Collision|EventActorBeginOverlap
  (params (OtherActor :type Actor%20Object%20Reference))
  (Utilities|FlowControl|Sequence
    (:then_0
      ;[0.15 0.15 0.15 0.5] Comment
      (bind _asbp_pcpuppet (Utilities|Casting|CastToBP_PCPuppet OtherActor))
      (bind _asbp_arcade_room_player_controller (Utilities|Casting|CastToBP_ArcadeRoomPlayerController (Pawn|GetController _asbp_pcpuppet)))
      (Default|AddPunchWidget _asbp_arcade_room_player_controller))
    (:then_1
      ;[0.15 0.15 0.15 0.5] Comment
      (bind _outactors (Actor|GetAllActorsOfClass "/Script/Engine.SpotLight"))
      (for _array_element _outactors
        (if (Utilities|String|Contains (Utilities|GetDisplayName _array_element) "Punch")
          (Rendering|SetVisibility (Variables|/Script/Engine.Light|GetLightComponent _array_element) true false))))))

(fn ConstructionScript)